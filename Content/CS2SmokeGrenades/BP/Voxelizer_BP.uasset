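; Voxelizer actor for CS2-style smoke grenades that divides a box volume into a voxel grid and visualizes how it fills.
; BeginPlay builds a flattened 3D array of box-relative voxel positions.
; DebugEvent resets it, then either marks voxels within a timeline-grown radius from the box's bottom center or replays already-flagged voxels, optionally with delayed loops.
; Filled voxels render as instanced meshes or random-colored debug boxes.
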(event Custom|DebugEvent
  (CallFunction|CleanFill)
  (if (Variables|Default|GetConstantFill%20)
    (|ConstantFillDebug)
    (else
      (|RadiusFillDebug))))

(event EventBeginPlay
  (VoxelArray|InitVoxelArray))

(event Collision|EventActorBeginOverlap
  (params (OtherActor :type Actor%20Object%20Reference)))

(event EventTick
  (params (DeltaSeconds :type Float%20%28single-precision%29)))

(fn ConstructionScript)

(fn InitVoxelArray
  (bind _voxelsize_ (Variables|Default|GetVoxelSize%20))
  (bind _box (Variables|Default|GetBox))
  (bind _voxelsize__2 (Variables|Default|GetVoxelSize%20))
  (bind _returnvalue (Components|Box|GetScaledBoxExtent _box))
  (bind _returnvalue_2 (* _returnvalue 2))
  ;[1 1 1] Init Voxel Size
  (Variables|Default|SetVoxelNumX (Math|Float|Truncate (/ (.x _returnvalue_2) _voxelsize__2)))
  (Variables|Default|SetVoxelNumY (Math|Float|Truncate (/ (.y _returnvalue_2) _voxelsize__2)))
  (Variables|Default|SetVoxelNumZ (Math|Float|Truncate (/ (.z _returnvalue_2) _voxelsize__2)))
  (Variables|Default|SetBoundsExtent%20 _returnvalue)
  ;[1 1 1] Init Voxel Array
  (Variables|VoxelArray|SetWidth (Variables|Default|GetVoxelNumX))
  (Variables|VoxelArray|SetDepth (Variables|Default|GetVoxelNumY))
  (Utilities|Array|Resize (Variables|VoxelArray|GetVoxel3DArray) (* (Variables|Default|GetVoxelNumX) (Variables|Default|GetVoxelNumY) (Variables|Default|GetVoxelNumZ)))
  (bind (_data _x _y _z) (Utilities|ForLoopVoxelData)
    (:then
      (|SetBy-RefVar _data (Utilities|Struct|MakeST_VoxelData false (- (Math|Vector|MakeVector (* _voxelsize_ _x) (* _voxelsize_ _y) (* _voxelsize_ _z)) (Components|Box|GetScaledBoxExtent (Variables|Default|GetBox))) 0)))
    (:Completed
      (return))))

(fn Debug
  (CallFunction|DebugEvent))

(fn FillRadius
  (params (Radius :type Float%20%28double-precision%29))
  (LocalVariables|SetRadius_ Radius)
  (for _index (range 0 (- (Variables|Default|GetVoxelNumX) 1))
    (for _index_2 (range 0 (- (Variables|Default|GetVoxelNumY) 1))
      (for _index_3 (range 0 (- (Variables|Default|GetVoxelNumZ) 1))
        (bind _index_4 (VoxelArray|Map3Dto1D _index _index_2 _index_3))
        (if (not (.HasVoxle (Utilities|Struct|BreakST_VoxelData (Utilities|Array|Get(acopy) (Variables|VoxelArray|GetVoxel3DArray) _index_4))))
          (if (<= (Math|Vector|VectorLength (/ (+ (.Position (Utilities|Struct|BreakST_VoxelData (Utilities|Array|Get(acopy) (Variables|VoxelArray|GetVoxel3DArray) _index_4))) (Math|Vector|MakeVector 0.0 0.0 (.z (Variables|Default|GetBoundsExtent%20)))) (Math|Vector|MakeVector (LocalVariables|GetRadius_) (LocalVariables|GetRadius_) (LocalVariables|GetRadius_)))) 1.0)
            (|SetBy-RefVar (Utilities|Array|Get(acopy) (Variables|VoxelArray|GetVoxel3DArray) _index_4) (Utilities|Struct|MakeST_VoxelData true (.Position (Utilities|Struct|BreakST_VoxelData (Utilities|Array|Get(acopy) (Variables|VoxelArray|GetVoxel3DArray) _index_4))) (.Power (Utilities|Struct|BreakST_VoxelData (Utilities|Array|Get(acopy) (Variables|VoxelArray|GetVoxel3DArray) _index_4)))))
            (CallFunction|Fill (.Position (Utilities|Struct|BreakST_VoxelData (Utilities|Array|Get(acopy) (Variables|VoxelArray|GetVoxel3DArray) _index_4)))))))))
  (return))

(fn Fill
  (params (Instance%20Transform%20Location :type Vector))
  (if (Variables|Default|GetIsDebug)
    ;[1 1 1] Debug
    (Rendering|Debug|DrawDebugBox (+ Instance%20Transform%20Location (Transformation|GetActorLocation)) (Math|Conversions|ToVector(Float) (- (/ (Variables|Default|GetVoxelSize%20) 2.0) 1.5)) (Math|Conversions|ToLinearColor(Vector) (Math|Random|RandomUnitVector)) "0, 0, 0" 5.0 3.0)
    (else
      (Components|InstancedStaticMesh|AddInstance (Variables|Default|GetInstancedStaticMesh) (Math|Transform|MakeTransform Instance%20Transform%20Location "0, 0, 0" "1.000000,1.000000,1.000000") false))))

(fn CleanFill
  (VoxelArray|InitVoxelArray)
  (Components|InstancedStaticMesh|ClearInstances (Variables|Default|GetInstancedStaticMesh)))

(fn Map3Dto1D
  (params (X :type Integer) (Y :type Integer) (Z :type Integer))
  (return (+ X (* (+ Y (* Z (Variables|VoxelArray|GetDepth))) (Variables|VoxelArray|GetWidth)))))

(fn Map1Dto3D
  (params (Index :type Integer))
  (bind _width (Variables|VoxelArray|GetWidth))
  (bind _depth (Variables|VoxelArray|GetDepth))
  (bind _returnvalue (* _width _depth))
  (bind _returnvalue_2 (/ Index _returnvalue))
  (return (Math|Integer|%(Integer) Index _width) (/ _width (* (- Index _returnvalue_2) _returnvalue)) _returnvalue_2))