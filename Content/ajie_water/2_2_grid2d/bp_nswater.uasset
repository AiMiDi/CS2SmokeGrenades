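; Niagara water actor in a Grid2D test that feeds the player pawn's position to the RT Niagara system.
; Tick, through a short Delay, wraps pawn XY into repeating 3000-unit tile UVs via Fraction and absolute value, sets User.position and prints it.
; Alternative writes to Niagara and material parameter collections are disconnected.
; A LocationToUV helper does the unwrapped division but is not called here.
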(event EventBeginPlay
  (Input|EnableInput (Game|GetPlayerController 0)))

(event Collision|EventActorBeginOverlap
  (params (OtherActor :type Actor%20Object%20Reference)))

(event EventTick
  (params (DeltaSeconds :type Float%20%28single-precision%29))
  (bind _returnvalue (Game|Player|GetPlayerPawn 0))
  (bind _returnvalue_2 (Transformation|GetActorLocation _returnvalue))
  (bind _returnvalue_3 (/ _returnvalue_2 "(X=3000.000000,Y=3000.000000)"))
  (bind (_x _y) (Math|Vector2D|BreakVector2D _returnvalue_3))
  (bind _returnvalue_4 (Math|Float|Fraction _y))
  (bind _returnvalue_5 (Math|Float|Fraction _x))
  (bind _returnvalue_6 (Math|Vector2D|MakeVector2D _returnvalue_5 _returnvalue_4))
  (bind _returnvalue_7 (Class|KismetMathLibrary|GetAbs2D _returnvalue_6))
  (Utilities|FlowControl|Delay 0.1)
  (Class|NiagaraComponent|SetVariableVec2 (Variables|Default|GetRT) "User.position" _returnvalue_7)
  (Development|PrintString (Utilities|String|ToString(Vector2d) _returnvalue_7)))

(fn ConstructionScript)

(fn LocationtoUV
  (params (position :type Vector))
  (bind (_x _y) (Math|Vector|BreakVector position))
  (return (/ (Math|Vector2D|MakeVector2D _x _y) "(X=3000.000000,Y=3000.000000)")))