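; Interactive water plane actor that simulates ripples where the player moves, using render targets.
; While a pawn overlaps it, Tick stamps the player's position (world XY/1000) into the current height target and feeds that to the water's WPO.
; HeightSim propagates waves across three cycling targets from the previous two frames, then ComputerNormal converts the result into the water normal map.
; Tick also writes player position and canvas size to MPC_water.
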(event EventBeginPlay
  (bind _waterplane (Variables|Default|Getwaterplane))
  ;[1 1 1] clearRT
  (Rendering|ClearRenderTarget2D "/Game/ajie_water/2_1_RT/Texture/H0.H0")
  (Rendering|ClearRenderTarget2D "/Game/ajie_water/2_1_RT/Texture/H1.H1")
  (Rendering|ClearRenderTarget2D "/Game/ajie_water/2_1_RT/Texture/H2.H2")
  (bind _returnvalue (Rendering|Material|CreateDynamicMaterialInstance _waterplane 0 "/Game/ajie_water/2_1_RT/Material/water.water" "" :!class /Script/Engine.PrimitiveComponent))
  (Variables|Default|Setwater_mid _returnvalue)
  (Rendering|Material|SetMaterial _waterplane 0 _returnvalue)
  (Rendering|Material|SetTextureParameterValue (Variables|Default|Getwater_mid) "waternormal" "/Game/ajie_water/2_1_RT/Texture/HeightFieldNormal.HeightFieldNormal"))

(event Collision|EventActorBeginOverlap
  (params (OtherActor :type Actor%20Object%20Reference))
  ;[1 1 1] 判断是否与pawn接触
  (bind _aspawn (Utilities|Casting|CastToPawn OtherActor)
    (:then
      _)
    (:CastFailed
      _))
  (if (not (== _aspawn 0))
    (Variables|Default|SetTouchingCharacter OtherActor)))

(event Collision|EventActorEndOverlap
  (params (OtherActor :type Actor%20Object%20Reference))
  ;[1 1 1] 判断是否与pawn接触
  (bind _aspawn (Utilities|Casting|CastToPawn OtherActor)
    (:then
      _)
    (:CastFailed
      _))
  (if (not (== _aspawn 0))
    (Variables|Default|SetTouchingCharacter 0)))

(event EventTick
  (params (DeltaSeconds :type Float%20%28single-precision%29))
  (bind _returnvalue (Game|Player|GetPlayerPawn 0))
  (bind _returnvalue_2 (Transformation|GetActorLocation _returnvalue))
  (bind _returnvalue_3 (CallFunction|LocationtoUV _returnvalue_2))
  (bind (_x _y) (Math|Vector2D|BreakVector2D _returnvalue_3))
  (CallFunction|RTPositiontoSeff)
  ;[1 1 1] 接触就开始传ForcePosition到RT上
  (if (== (Variables|Default|GetTouchingCharacter) 0)
    _
    (else
      (bind _lastrt (CallFunction|GetRT (Variables|Default|Getrt_num)))
      ;[1 1 1] 设置传点的材质
      (bind _returnvalue_4 (Rendering|Material|CreateDynamicMaterialInstance "/Game/ajie_water/2_1_RT/Material/ForcePosition.ForcePosition" "None" "None" :!class /Script/Engine.KismetMaterialLibrary))
      ;[1 1 1] 将人物世界坐标转到uv空间坐标
      (Rendering|Material|SetVectorParameterValue _returnvalue_4 "ForcePosition" (Math|Conversions|ToLinearColor(Vector) (Math|Vector|MakeVector _x _y 0.0)) :!class /Script/Engine.MaterialInstanceDynamic)
      (Rendering|DrawMaterialtoRenderTarget _lastrt _returnvalue_4)
      ;[1 1 1] 设置水面材质的wpo
      (Rendering|Material|SetTextureParameterValue (Variables|Default|Getwater_mid) "wpo" _lastrt)))
  (Utilities|FlowControl|Sequence
    (:then_0
      ;[1 1 1] sim扩散模拟
      ;;[1 1 1] 设置rt循环
      (Variables|Default|Setrt_num (Math|Integer|%(Integer) (+ (Variables|Default|Getrt_num) 1) 3))
      ;;[1 1 1] 设置扩散材质
      (bind _returnvalue_5 (Rendering|Material|CreateDynamicMaterialInstance "/Game/ajie_water/2_1_RT/Material/HeightSim.HeightSim" "None" "None" :!class /Script/Engine.KismetMaterialLibrary))
      ;;[1 1 1] 获取上一张rt
      (bind _lastrt_2 (CallFunction|GetLastHeight (Variables|Default|Getrt_num) 1))
      ;;[1 1 1] 设置到sim材质的height1
      (Rendering|Material|SetTextureParameterValue _returnvalue_5 "PreviousHeight1" _lastrt_2)
      ;;[1 1 1] 获取上上张rt
      (bind _lastrt_3 (CallFunction|GetLastHeight (Variables|Default|Getrt_num) 2))
      ;;[1 1 1] 设置到sim材质的heght2
      (Rendering|Material|SetTextureParameterValue _returnvalue_5 "PreviousHeight2" _lastrt_3)
      ;;[1 1 1] 绘制当前rt
      (bind _lastrt_4 (CallFunction|GetRT (Variables|Default|Getrt_num)))
      (bind (_canvas _size _context) (Rendering|BeginDrawCanvastoRenderTarget _lastrt_4))
      (Canvas|DrawMaterial :self _canvas :RenderMaterial _returnvalue_5 :ScreenSize _size :CoordinateSize "(X=1.000000,Y=1.000000)" :PivotPoint "(X=0.500000,Y=0.500000)")
      (Rendering|EndDrawCanvastoRenderTarget _context))
    (:then_1
      ;[1 1 1] 创建法线材质
      (bind _returnvalue_6 (Rendering|Material|CreateDynamicMaterialInstance "/Game/ajie_water/2_1_RT/Material/computerNormal.computerNormal" "None" "None" :!class /Script/Engine.KismetMaterialLibrary))
      ;[1 1 1] 获取当前rt
      (bind _lastrt_5 (CallFunction|GetRT (Variables|Default|Getrt_num)))
      ;[1 1 1] 将rt传到computerNormal上，然后转化为normal图
      (Rendering|Material|SetTextureParameterValue _returnvalue_6 "normal" _lastrt_5)
      ;[1 1 1] 将扩散normal图传到新的输出的rt上
      (Rendering|DrawMaterialtoRenderTarget "/Game/ajie_water/2_1_RT/Texture/HeightFieldNormal.HeightFieldNormal" _returnvalue_6)
      ;[1 1 1] 传到水面材质的法线上
      (Rendering|Material|SetTextureParameterValue (Variables|Default|Getwater_mid) "waternormal" "/Game/ajie_water/2_1_RT/Texture/HeightFieldNormal.HeightFieldNormal"))
    (:then_2
      (Development|PrintString (Utilities|String|ToString(Vector2d) _returnvalue_3)))))

(fn ConstructionScript)

(fn LocationtoUV
  (params (position :type Vector))
  (bind (_x _y) (Math|Vector|BreakVector position))
  (return (/ (Math|Vector2D|MakeVector2D _x _y) "(X=1000.000000,Y=1000.000000)")))

(fn GetRT
  (params (num :type Integer))
  (if (== num 0)
    (return "/Game/ajie_water/2_1_RT/Texture/H0.H0")
    (elif (== num 1)
      (return "/Game/ajie_water/2_1_RT/Texture/H1.H1")
      (else
        (return "/Game/ajie_water/2_1_RT/Texture/H2.H2")))))

(fn GetLastHeight
  (params (CurrentHeightIndex :type Integer) (NumFramesOld :type Integer))
  (bind _lastrt (CallFunction|GetRT (Math|Integer|%(Integer) (+ (- CurrentHeightIndex NumFramesOld) 3) 3)))
  (return _lastrt))

(fn RTPositiontoSeff
  (bind _canvasszie (Variables|Default|GetCanvasSzie))
  (bind (_x _y) (Math|Vector2D|BreakVector2D _canvasszie))
  (bind _output_get (Variables|Default|SetCanvasPosition (Math|Conversions|ToVector2D(Vector) (Transformation|GetActorLocation (Game|Player|GetPlayerPawn 0)))))
  (Rendering|Material|SetVectorParameterValue "/Game/ajie_water/2_1_RT/Material/MPC_water.MPC_water" "Position" (Utilities|Struct|MakeLinearColor (.X (Math|Vector2D|BreakVector2D _output_get)) (.Y (Math|Vector2D|BreakVector2D _output_get)) _x _y) :!class /Script/Engine.KismetMaterialLibrary))

(fn TransformPositiontoRT
  (params (Positon :type Vector%202D%20Structure))
  (return (+ (/ (- Positon (Variables|Default|GetCanvasPosition)) (Variables|Default|GetCanvasSzie)) "(X=0.500000,Y=0.500000)")))